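; Inventory component that stores items by name in an array, capped at three through AddItem, and seeds it with a "Key" at BeginPlay.
; AddItem tracks a running ItemsCount and reports whether the add succeeded, printing a message when full.
; CheckForItem searches the array for a name, and ShowInventory prints its contents.
; CountItems adds the array length onto ItemsCount without resetting it, printing each step.
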(event `self.ReceiveBeginPlay`
  (`self.addItem` "Key"))

(fn `addItem`
  (params (item :type String))
  (returns (isntFull :type Boolean) (itemCount :type Integer))
  (set `self.itemName` item)
  (if (> (`self.ItemsCount`) 2)
    (`KismetSystemLibrary.PrintString` "Inventory Full!")
    (return false (`self.ItemsCount`))
    (else
      (set `self.ItemsCount` (+ (`self.ItemsCount`) 1))
      (`KismetArrayLibrary.Array_Add` (`self.Inventory`) (`self.itemName`))
      (return true (`self.ItemsCount`)))))

(fn `CheckForItem`
  (params (ItemNameToCheck :type String))
  (returns (HasIte :type Boolean))
  (bind _returnvalue (`KismetArrayLibrary.Array_Length` (`self.Inventory`)))
  (if (== _returnvalue 0)
    (return false)
    (else
      (for _index (range (+ _returnvalue 1))
        (if (`KismetStringLibrary.EqualEqual_StrStr` (`|GetArrayItem` (`self.Inventory`) _index) (`local.ItemNameToCheck`))
          (return true)))
      (return false))))

(fn `CountItems`
  (returns (IsntFull :type Boolean) (count :type Integer))
  (for _ (`self.Inventory`)
    (bind _output_get (set `self.ItemsCount` (+ 1 (`self.ItemsCount`))))
    (`KismetSystemLibrary.PrintString` (`KismetStringLibrary.Conv_IntToString` _output_get) true true (struct :`R` 0.983455 :`G` 1.0 :`B` 0.946885 :`A` 1.0) 25.0))
  (if (> (`self.ItemsCount`) 2)
    (`KismetSystemLibrary.PrintString` "Inventory Full!")
    (return false (`self.ItemsCount`))
    (else
      (return true 0))))

(fn `showInventory`
  (for _array_element (`self.Inventory`)
    (`KismetSystemLibrary.PrintString` _array_element)))