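; Dog actor Blueprint whose skeletal mesh can be made happy and then moved to a preset teleport spot.
; On BeginPlay it caches the mesh's ABP_dog animation instance, and MAkeHappy sets that instance's IsHappy flag.
; Each Tick, when the anim instance reports both IsHappy and ShouldTeleport, Teleport snaps the mesh to the TeleportLocation component's world position without sweeping.
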(event `self.ReceiveBeginPlay`
  (bind _asabp_dog (cast `/Game/Art/animaux/ABP_dog` (`SkeletalMeshComponent.GetAnimInstance` (`self.SKM_Dawgg`))))
  (set `self.ABP_Dog` _asabp_dog))

(event `self.ReceiveTick`
  (params (DeltaSeconds :type "Float (single-precision)"))
  (bind _abp_dog (`self.ABP_Dog`))
  (if (and (`/Game/Art/animaux/ABP_dog.isHappy` _abp_dog) (`/Game/Art/animaux/ABP_dog.ShouldTeleport` _abp_dog))
    (`self.Teleport`)))

(fn `MAke Happy`
  (set `/Game/Art/animaux/ABP_dog.isHappy` true (`self.ABP_Dog`)))

(fn `Teleport`
  (`SceneComponent.K2_SetWorldLocation` (`self.SKM_Dawgg`) (`SceneComponent.K2_GetComponentLocation` (`self.TeleportLocation`)) false false))

(fn `UserConstructionScript`)