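; Player character that moves, talks to NPCs, collects items and gathers souls, with a resources widget on screen.
; Each tick, health components heal it inside the cult radius or a key object's overlap and damage it elsewhere.
; A per-tick sphere overlap caches the nearest BP_Items actor for the interact input, which also triggers NPC dialogue.
; Equipped item meshes attach to hand sockets, right first, and soul gains fire a notification.
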(event `self.ReceiveBeginPlay`
  (bind _returnvalue (`|CreateWidget` "/Game/UI/WB_Ressources.WB_Ressources_C" (`GameplayStatics.GetPlayerController` 0)))
  (`UserWidget.AddToViewport` _returnvalue 0))

(event `self.ReceiveTick`
  (params (DeltaSeconds :type "Float (single-precision)"))
  (bind _cbp_player_health (`self.CBP_Player_Health`))
  (bind _returnvalue (`SceneComponent.K2_GetComponentLocation` (`self.Mesh`)))
  (`|ExecutionSequence`
    (:`then_0`
      (bind _iskeyobjectinsideradius (`/Game/Blueprint/Player/CBP_Player_CultRadius.CalculateCultRaadius` (`self.CBP_Player_CultRadius`) _returnvalue))
      (if _iskeyobjectinsideradius
        (`/Game/Blueprint/Player/CBP_Player_Health.ResetDamageCounter` _cbp_player_health :!label _label)
        (`/Game/Blueprint/Player/CBP_Player_Health.ResetGracePeriod` _cbp_player_health)
        (`/Game/Blueprint/Player/CBP_Player_Health.Heal` _cbp_player_health 0.1 1.0)
        (elif (`self.IsInKeyObjectRadius`)
          (goto _label)
          (else
            (`/Game/Blueprint/Player/CBP_Player_Health.ResetHealthTimer` _cbp_player_health)
            (`/Game/Blueprint/Player/CBP_Player_Health.TakeDamage` _cbp_player_health 0.1 1.0))))
      (`/Game/Blueprint/Player/CBP_Player_Health.PrintLogs` (`self.CBP_Player_Health`)))
    (:`then_1`
      (bind (_outactors _returnvalue_2) (`KismetSystemLibrary.SphereOverlapActors` _returnvalue 200.0 (`|MakeArray` "ObjectTypeQuery1" :!type "EObjectTypeQuery Enum") "/Game/Blueprint/Objects/Inventory/BP_Items.BP_Items_C"))
      (if _returnvalue_2
        (bind _asbp_items (cast `/Game/Blueprint/Objects/Inventory/BP_Items` (`.ReturnValue` (`GameplayStatics.FindNearestActor` _returnvalue _outactors))))
        (set `self.ClosestObject` _asbp_items)
        (else
          (set `self.ClosestObject` null))))))

(event `self.ReceiveActorBeginOverlap`
  (params (OtherActor :type "Actor Object Reference"))
  (bind _cbp_player_health (`self.CBP_Player_Health`))
  (cast `/Game/Blueprint/Gameplay/BP_KeyObject` OtherActor)
  (set `self.IsInKeyObjectRadius` true)
  (`/Game/Blueprint/Player/CBP_Player_Health.ResetDamageCounter` _cbp_player_health)
  (`/Game/Blueprint/Player/CBP_Player_Health.ResetGracePeriod` _cbp_player_health))

(event `self.ReceiveActorEndOverlap`
  (params (OtherActor :type "Actor Object Reference"))
  (cast `/Game/Blueprint/Gameplay/BP_KeyObject` OtherActor)
  (set `self.IsInKeyObjectRadius` false))

(event `EnhancedInput|/Game/TopDown/Input/Actions/IA_MoveAround`
  (params (ActionValue :type "Vector2D Structure") (ElapsedSeconds :type "Float (double-precision)") (TriggeredSeconds :type "Float (double-precision)") (InputAction :type "InputAction Object Reference" :default "/Game/TopDown/Input/Actions/IA_MoveAround.IA_MoveAround"))
  (:`Triggered`
    (if (not (`self.IsDialoguing`))
      (`self.AddMovementInput` (0.0 1.0 0.0) ActionValue_X)
      (`self.AddMovementInput` (1.0 0.0 0.0) ActionValue_Y))))

(event `EnhancedInput|/Game/TopDown/Input/Actions/IA_Interact`
  (params (ActionValue :type Boolean) (ElapsedSeconds :type "Float (double-precision)") (TriggeredSeconds :type "Float (double-precision)") (InputAction :type "InputAction Object Reference" :default "/Game/TopDown/Input/Actions/IA_Interact.IA_Interact"))
  (bind _npc (`self.NPC`))
  (bind _closestobject (`self.ClosestObject`))
  (:`Started`
    (`|ExecutionSequence`
      (:`then_0`
        (if (`KismetSystemLibrary.IsValid` _npc)
          (`/Game/Blueprint/NPCs/BP_NPCTest.TryDialogue` _npc)))
      (:`then_1`
        (if (`KismetSystemLibrary.IsValid` _closestobject)
          (`/Game/Blueprint/Objects/Inventory/BP_Items.TryCollectObject` _closestobject))))))

(event `EnhancedInput|/Game/TopDown/Input/Actions/IA_ContinuerDialogue`
  (params (ActionValue :type Boolean) (ElapsedSeconds :type "Float (double-precision)") (TriggeredSeconds :type "Float (double-precision)") (InputAction :type "InputAction Object Reference" :default "/Game/TopDown/Input/Actions/IA_ContinuerDialogue.IA_ContinuerDialogue"))
  (bind _npc (`self.NPC`))
  (:`Started`
    (if (`KismetSystemLibrary.IsValid` _npc)
      (`/Game/Blueprint/NPCs/BP_NPCTest.HandleDialogue` _npc))))

(fn `AddSoul`
  (params (Amount :type Integer))
  (bind _output_get (set `self.SoulAmount` (+ Amount (`self.SoulAmount`))))
  (`self.OnSoulObtained` _output_get))

(fn `ChangeSpeed`
  (params (value :type "Float (double-precision)"))
  (set `CharacterMovementComponent.MaxWalkSpeed` value (`self.CharacterMovement`)))

(fn `Equip Item`
  (params (Object :type "/Game/Blueprint/Objects/Inventory/BP_Items Object Reference"))
  (bind _item_r (`self.Item_R`))
  (bind _item_l (`self.Item_L`))
  (bind _itemmesh (`/Game/Blueprint/Objects/Inventory/BP_Items.ItemMesh` Object))
  (`KismetSystemLibrary.PrintString` (`KismetStringLibrary.Concat_StrStr` "AAAA " (`/Game/Blueprint/Objects/Inventory/BP_Items.ItemName` Object)))
  (if (`self.rightHandFull`)
    (`StaticMeshComponent.SetStaticMesh` _item_l _itemmesh)
    (`PrimitiveComponent.SetMaterial` _item_l 0 (`StaticMesh.GetMaterial` _itemmesh 0))
    (`SceneComponent.K2_AttachToComponent` _item_l (`self.Mesh`) "handSocket_L" "KeepRelative" "KeepRelative" "KeepWorld" true)
    (else
      (`StaticMeshComponent.SetStaticMesh` _item_r _itemmesh)
      (`PrimitiveComponent.SetMaterial` _item_r 0 (`StaticMesh.GetMaterial` _itemmesh 0))
      (`SceneComponent.K2_AttachToComponent` (`self.Item_R`) (`self.Mesh`) "handSocket_R" "KeepRelative" "KeepRelative" "KeepWorld" true)
      (set `self.rightHandFull` true))))

(fn `IsTalking`
  (params (IsDialoguing :type Boolean))
  (set `self.IsDialoguing` IsDialoguing))

(fn `Unequip Item`
  (params (ObjectName :type String))
  (bind _bpc_inventory (`self.BPC_Inventory`))
  (if (`KismetStringLibrary.IsEmpty` (`/Game/Blueprint/Objects/Inventory/Components/BPC_Inventory.ObjecNametInRightHand` _bpc_inventory))
    (`SceneComponent.K2_DetachFromComponent` (`self.Item_R`) "KeepRelative" "KeepRelative" "KeepWorld" true)
    (elif (`KismetStringLibrary.IsEmpty` (`/Game/Blueprint/Objects/Inventory/Components/BPC_Inventory.ObjecNametInLeftHand` _bpc_inventory))
      (`SceneComponent.K2_DetachFromComponent` (`self.Item_L`) "KeepRelative" "KeepRelative" "KeepRelative" true)
      (else
        (`KismetSystemLibrary.PrintString` "OMG FUCJING WORK!!!!!!! SHITY UE!!!!!!" true true (struct :`R` 1.0 :`A` 1.0))))))

(fn `UserConstructionScript`)