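; Player character that creates the resources widget, moves with Enhanced Input except during dialogue, and tracks collected souls.
; Each Tick, the cult radius component checks its position: inside that radius or a key object's overlap, the health component heals; otherwise it applies damage.
; Helpers set walk speed, toggle dialogue state, broadcast soul gains, and attach items to hand sockets, right hand first.
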(event `self.ReceiveBeginPlay`
  (bind _returnvalue (`|CreateWidget` "/Game/UI/WB_Ressources.WB_Ressources_C" (`GameplayStatics.GetPlayerController` 0)))
  (`UserWidget.AddToViewport` _returnvalue 0)
  (bind _returnvalue_2 (`GameplayStatics.GetActorOfClass` "/Game/Blueprint/NPCs/BP_NPCTest.BP_NPCTest_C"))
  (set `self.NPC` _returnvalue_2))

(event `self.ReceiveTick`
  (params (DeltaSeconds :type "Float (single-precision)"))
  (bind _cbp_player_health (`self.CBP_Player_Health`))
  (bind _iskeyobjectinsideradius (`/Game/Blueprint/Player/CBP_Player_CultRadius.CalculateCultRaadius` (`self.CBP_Player_CultRadius`) (`SceneComponent.K2_GetComponentLocation` (`self.Mesh`))))
  (if _iskeyobjectinsideradius
    (`/Game/Blueprint/Player/CBP_Player_Health.ResetDamageCounter` _cbp_player_health :!label _label)
    (`/Game/Blueprint/Player/CBP_Player_Health.ResetGracePeriod` _cbp_player_health)
    (`/Game/Blueprint/Player/CBP_Player_Health.Heal` _cbp_player_health 0.1 1.0)
    (elif (`self.IsInKeyObjectRadius`)
      (goto _label)
      (else
        (`/Game/Blueprint/Player/CBP_Player_Health.ResetHealthTimer` _cbp_player_health)
        (`/Game/Blueprint/Player/CBP_Player_Health.TakeDamage` _cbp_player_health 0.1 1.0))))
  (`/Game/Blueprint/Player/CBP_Player_Health.PrintLogs` (`self.CBP_Player_Health`)))

(event `self.ReceiveActorBeginOverlap`
  (params (OtherActor :type "Actor Object Reference"))
  (bind _cbp_player_health (`self.CBP_Player_Health`))
  (cast `/Game/Blueprint/Gameplay/BP_KeyObject` OtherActor)
  (set `self.IsInKeyObjectRadius` true)
  (`/Game/Blueprint/Player/CBP_Player_Health.ResetDamageCounter` _cbp_player_health)
  (`/Game/Blueprint/Player/CBP_Player_Health.ResetGracePeriod` _cbp_player_health))

(event `self.ReceiveActorEndOverlap`
  (params (OtherActor :type "Actor Object Reference"))
  (cast `/Game/Blueprint/Gameplay/BP_KeyObject` OtherActor)
  (set `self.IsInKeyObjectRadius` false))

(event `EnhancedInput|/Game/TopDown/Input/Actions/IA_MoveAround`
  (params (ActionValue :type "Vector2D Structure") (ElapsedSeconds :type "Float (double-precision)") (TriggeredSeconds :type "Float (double-precision)") (InputAction :type "InputAction Object Reference" :default "/Game/TopDown/Input/Actions/IA_MoveAround.IA_MoveAround"))
  (:`Triggered`
    (if (not (`self.IsDialoguing`))
      (`self.AddMovementInput` (0.0 1.0 0.0) ActionValue_X)
      (`self.AddMovementInput` (1.0 0.0 0.0) ActionValue_Y))))

(fn `AddSoul`
  (params (Amount :type Integer))
  (bind _output_get (set `self.SoulAmount` (+ Amount (`self.SoulAmount`))))
  (`self.OnSoulObtained` _output_get))

(fn `ChangeSpeed`
  (params (value :type "Float (double-precision)"))
  (set `CharacterMovementComponent.MaxWalkSpeed` value (`self.CharacterMovement`)))

(fn `EquipItem`
  (params (Mesh :type "StaticMesh Object Reference") (itemCount :type Integer))
  (bind _item (`self.Item`))
  (set `self.itemCount` itemCount)
  (`StaticMeshComponent.SetStaticMesh` _item Mesh)
  (`PrimitiveComponent.SetMaterial` _item 0 (`StaticMesh.GetMaterial` Mesh 0))
  (if (`self.rightHandFull`)
    (`SceneComponent.K2_AttachToComponent` (`self.Item`) (`self.Mesh`) "handSocket_L" "SnapToTarget" "SnapToTarget" "KeepRelative" true)
    (set `self.leftHandFull` true)
    (else
      (`SceneComponent.K2_AttachToComponent` (`self.Item`) (`self.Mesh`) "handSocket_R" "SnapToTarget" "SnapToTarget" "KeepRelative" true)
      (set `self.rightHandFull` true))))

(fn `IsTalking`
  (params (IsDialoguing :type Boolean))
  (set `self.IsDialoguing` IsDialoguing))

(fn `UserConstructionScript`)