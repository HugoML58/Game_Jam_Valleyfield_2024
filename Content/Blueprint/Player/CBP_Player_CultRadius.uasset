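; Player cult-radius Blueprint that finds sub key objects around a position and handles their collection.
; CalculateCultRaadius draws a debug sphere at CultRadius and returns the WorldStatic BP_SubKeyObject actors overlapping it.
; TryCollectObject destroys an actor passed to it if it is a BP_SubKeyObject, and AgmentCultRadius adds a value to the radius.
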(fn `AgmentCultRadius`
  (params (ValueToAdd :type "Float (double-precision)"))
  (set `self.CultRadius` (+ ValueToAdd (`self.CultRadius`))))

(fn `CalculateCultRaadius`
  (params (PlayerPosition :type "Vector Structure"))
  (returns (IsKeyObjectInsideRadius :type Boolean))
  (bind _cultradius (`self.CultRadius`))
  (`|ExecutionSequence`
    (:`then_0`
      (`KismetSystemLibrary.DrawDebugSphere` PlayerPosition _cultradius))
    (:`then_1`
      (bind (_outactors _returnvalue) (`KismetSystemLibrary.SphereOverlapActors` PlayerPosition _cultradius (`|MakeArray` "ObjectTypeQuery1" :!type "EObjectTypeQuery Enum") "/Game/Blueprint/Objects/BP_SubKeyObject.BP_SubKeyObject_C"))
      (return _returnvalue))))

(fn `TryCollectObject`
  (params (Other :type "Actor Object Reference"))
  (bind _asbp_sub_key_object (cast `/Game/Blueprint/Objects/BP_SubKeyObject` Other))
  (`Actor.K2_DestroyActor` _asbp_sub_key_object))