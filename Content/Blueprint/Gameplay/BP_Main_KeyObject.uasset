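; BP_Main_KeyObject is a key gameplay object with a sphere and decal area that grows as the player obtains souls.
; On BeginPlay it applies its starting radius and binds to the OnSoulObtained event of BP_Player1.
; Each soul amount feeds AddRadius2, which increases Radius, resizes the sphere with overlap updates and scales the decal to match.
; A debug print remains in AddRadius2, and the AddRadius event is empty.
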(event `self.ReceiveBeginPlay`
  (`self.AddRadius2` 0.0)
  (bind _asbp_player_1 (cast `/Game/Blueprint/Player/BP_Player1` (`GameplayStatics.GetPlayerCharacter` 0)))
  (add `/Game/Blueprint/Player/BP_Player1.OnSoulObtained` _asbp_player_1 (delegate `AugmentRadius`)))

(event `AugmentRadius`
  (params (Amount :type Integer))
  (`self.AddRadius2` (`KismetMathLibrary.Conv_IntToDouble` Amount)))

(event `/Game/Blueprint/Gameplay/BPI_KeyObject.AddRadius`
  (params (ValueToAdd :type "Float (double-precision)")))

(fn `AddRadius2`
  (params (NewParam :type "Float (double-precision)"))
  (bind _returnvalue (/ (`self.Radius`) 250.0))
  (`KismetSystemLibrary.PrintString` "awdfawfawfaw")
  (bind _output_get (set `self.Radius` (+ NewParam (`self.Radius`))))
  (`SphereComponent.SetSphereRadius` (`self.Sphere`) _output_get true)
  (`SceneComponent.SetRelativeScale3D` (`self.Decal`) (`KismetMathLibrary.MakeVector` 0.5 _returnvalue _returnvalue)))

(fn `UserConstructionScript`)