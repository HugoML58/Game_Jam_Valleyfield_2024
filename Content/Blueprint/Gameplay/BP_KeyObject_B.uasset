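; BP_KeyObject_B is a key object actor with a radius-driven sphere area and a decal; the file defines no interaction logic.
; On BeginPlay, the Radius variable sets the Sphere component's size, updating overlaps, and scales the Decal's Y and Z to match while its X scale stays fixed.
; Every Tick it draws a debug sphere of that radius at the actor's location.
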(event `self.ReceiveBeginPlay`
  (bind _returnvalue (/ (`self.Radius`) 250.0))
  (`SphereComponent.SetSphereRadius` (`self.Sphere`) (`self.Radius`) true)
  (`SceneComponent.SetRelativeScale3D` (`self.Decal`) (`KismetMathLibrary.MakeVector` 0.5 _returnvalue _returnvalue)))

(event `self.ReceiveTick`
  (params (DeltaSeconds :type "Float (single-precision)"))
  (`KismetSystemLibrary.DrawDebugSphere` (`self.K2_GetActorLocation`) (`self.Radius`)))

(fn `UserConstructionScript`)