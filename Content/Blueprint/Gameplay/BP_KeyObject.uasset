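; BP_KeyObject is a world object with a circular area of influence that expands as the player obtains souls.
; On BeginPlay it binds to the player's OnSoulObtained event, adding the received amount to its Radius.
; AddRadius resizes the Sphere component and scales the Decal to match, keeping the overlap area and its visual in sync.
; Tick draws a debug sphere at the current radius.
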(event `self.ReceiveBeginPlay`
  (`self.AddRadius` 0.0)
  (bind _asbp_player (cast `/Game/Blueprint/Player/BP_Player` (`GameplayStatics.GetPlayerCharacter` 0)))
  (set `self.PlayerRef` _asbp_player)
  (add `/Game/Blueprint/Player/BP_Player.OnSoulObtained` (`self.PlayerRef`) (delegate `AugmentRadius`)))

(event `AugmentRadius`
  (params (Amount :type Integer))
  (`self.AddRadius` (`KismetMathLibrary.Conv_IntToDouble` Amount)))

(event `self.ReceiveTick`
  (params (DeltaSeconds :type "Float (single-precision)"))
  (`KismetSystemLibrary.DrawDebugSphere` (`self.K2_GetActorLocation`) (`self.Radius`)))

(fn `AddRadius`
  (params (ValueToAdd :type "Float (double-precision)"))
  (bind _returnvalue (/ (`self.Radius`) 250.0))
  (bind _output_get (set `self.Radius` (+ ValueToAdd (`self.Radius`))))
  (`SphereComponent.SetSphereRadius` (`self.Sphere`) _output_get true)
  (`SceneComponent.SetRelativeScale3D` (`self.Decal`) (`KismetMathLibrary.MakeVector` 1.0 _returnvalue _returnvalue)))

(fn `UserConstructionScript`)