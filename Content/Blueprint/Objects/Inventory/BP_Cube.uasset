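; BP_Cube is a purchasable world object that the player buys by touching it.
; BeginPlay sets its name and cost, so duplicated classes can become other items easily.
; On Sphere overlap with BP_Player, it compares the player's BPCMoney balance to the cost, then adds its name to BPCInventory and destroys itself, or prints a failure message.
; The graph checks the balance but never calls anything to deduct the cost.
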(event `self.ReceiveBeginPlay`
  ;[0.000938 0 0.02083] Init variables so its easier when we dupe this class
  (set `self.Cost` 20)
  (set `self.Name` "Cube"))

(event `self.Sphere.OnComponentBeginOverlap`
  (params (OverlappedComponent :type "PrimitiveComponent Object Reference") (OtherActor :type "Actor Object Reference") (OtherComp :type "PrimitiveComponent Object Reference") (OtherBodyIndex :type Integer) (bFromSweep :type Boolean) (SweepResult :type "HitResult Structure (by ref)"))
  (bind _asbp_player (cast `/Game/TopDown/Blueprints/BP_Player` OtherActor))
  (bind _money (`/Game/Blueprint/Player/BPC_Money.outputMoney` (`/Game/TopDown/Blueprints/BP_Player.BPC_Money` _asbp_player)))
  (if (>= _money (`self.Cost`))
    (`/Game/Blueprint/Objects/Inventory/Components/BPC_Inventory.addItem` (`/Game/TopDown/Blueprints/BP_Player.BPC_Inventory` _asbp_player) (`self.Name`))
    (`KismetSystemLibrary.PrintString` "Bought")
    (`self.K2_DestroyActor`)
    (else
      (`KismetSystemLibrary.PrintString` "ur broke"))))

(fn `UserConstructionScript`)