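; BP_Items_2 is a collectible item actor that shows a configurable mesh and can be picked up by BP_Player1.
; Sphere overlap with the player toggles the mesh's custom depth rendering and a proximity flag.
; When close, TryCollectObject calls the inventory component's AddItem; on a false return it equips the item and destroys the actor.
; Boots additionally change the player's speed before destruction.
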(event `self.ReceiveBeginPlay`
  (bind _cube (`self.Cube`))
  (bind _itemmesh (`self.ItemMesh`))
  (`StaticMeshComponent.SetStaticMesh` _cube _itemmesh)
  (`PrimitiveComponent.SetMaterial` _cube 0 (`StaticMesh.GetMaterial` _itemmesh 0))
  (bind _returnvalue (`GameplayStatics.GetActorOfClass` "/Game/Blueprint/Player/BP_Player1.BP_Player1_C"))
  (set `self.Player` _returnvalue))

(event `self.Sphere.OnComponentBeginOverlap`
  (params (OverlappedComponent :type "PrimitiveComponent Object Reference") (OtherActor :type "Actor Object Reference") (OtherComp :type "PrimitiveComponent Object Reference") (OtherBodyIndex :type Integer) (bFromSweep :type Boolean) (SweepResult :type "HitResult Structure (by ref)"))
  (cast `/Game/Blueprint/Player/BP_Player1` OtherActor)
  (`PrimitiveComponent.SetRenderCustomDepth` (`self.Cube`) true)
  (set `self.isClose` true))

(event `self.Sphere.OnComponentEndOverlap`
  (params (OverlappedComponent :type "PrimitiveComponent Object Reference") (OtherActor :type "Actor Object Reference") (OtherComp :type "PrimitiveComponent Object Reference") (OtherBodyIndex :type Integer))
  (cast `/Game/Blueprint/Player/BP_Player1` OtherActor)
  (`PrimitiveComponent.SetRenderCustomDepth` (`self.Cube`) false)
  (set `self.isClose` false))

(fn `TryCollectObject`
  (bind _itemname (`self.ItemName`))
  (if (`self.isClose`)
    (bind _isinventoryfull (`/Game/Blueprint/Objects/Inventory/Components/BPC_Inventory.addItem` (`/Game/Blueprint/Player/BP_Player1.BPC_Inventory` (`self.Player`)) _itemname))
    (if (not _isinventoryfull)
      (`/Game/Blueprint/Player/BP_Player1.Equip Item` (`self.Player`) self)
      (switch `string` _itemname
        (:`Default`
          (`self.K2_DestroyActor`))
        (:`Boots`
          (`/Game/Blueprint/Player/BP_Player1.ChangeSpeed` (`self.Player`) 1000.0)
          (`self.K2_DestroyActor`))))))

(fn `UserConstructionScript`)