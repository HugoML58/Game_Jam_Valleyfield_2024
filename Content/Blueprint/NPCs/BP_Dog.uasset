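; Dog NPC that the player can pet and that teleports away once its quest is completed.
; Interacting nearby plays a petting montage on the player, provided no dialogue is active and the quest is unfinished.
; Continuing dialogue nearby arms teleportation; releasing that input after dialogue ends with the quest complete triggers the dog AnimBP's heaven event.
; After a delay, its root moves to the TeleportationPoint found at BeginPlay.
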(event `self.ReceiveBeginPlay`
  (bind _returnvalue (`GameplayStatics.GetActorOfClass` "/Game/Blueprint/NPCs/TeleportationPoint.TeleportationPoint_C"))
  (set `self.As Teleportation Point` _returnvalue)
  (bind _asabp_dog (cast `/Game/Art/animaux/ABP_dog` (`SkeletalMeshComponent.GetAnimInstance` (`self.SkeletalMesh`))))
  (set `self.As ABP Dog` _asabp_dog)
  (`parent.ReceiveBeginPlay`))

(event `EnhancedInput|/Game/TopDown/Input/Actions/IA_Interact`
  (params (ActionValue :type Boolean) (ElapsedSeconds :type "Float (double-precision)") (TriggeredSeconds :type "Float (double-precision)") (InputAction :type "InputAction Object Reference" :default "/Game/TopDown/Input/Actions/IA_Interact.IA_Interact"))
  (:`Triggered`
    (if (not (or (`self.IsInDialogue`) (`self.HasCompletedQuest`) (not (`self.IsClose`))))
      (`AnimInstance.PlaySlotAnimationAsDynamicMontage` (`SkeletalMeshComponent.GetAnimInstance` (`Character.Mesh` (`self.Player`))) "/Game/Characters/bobbleCharacters/player/animations/SK_char_petting.SK_char_petting" "PettingDog" 0.25 0.25 1.0 1 -1.0 0.0))))

(event `EnhancedInput|/Game/TopDown/Input/Actions/IA_ContinuerDialogue`
  (params (ActionValue :type Boolean) (ElapsedSeconds :type "Float (double-precision)") (TriggeredSeconds :type "Float (double-precision)") (InputAction :type "InputAction Object Reference" :default "/Game/TopDown/Input/Actions/IA_ContinuerDialogue.IA_ContinuerDialogue"))
  (:`Triggered`
    (if (and (`self.IsInDialogue`) (`self.IsClose`))
      (set `self.CanTeleport` true)))
  (:`Completed`
    (if (and (== (`self.IsInDialogue`) false) (`self.CanTeleport`) (`self.HasCompletedQuest`))
      (`/Game/Art/animaux/ABP_dog.DoginHeaven` (`self.As ABP Dog`))
      (`KismetSystemLibrary.Delay` 5.0)
      (`KismetSystemLibrary.PrintString` "I'm gaming")
      (`self.Teleport`))))

(fn `Teleport`
  (`SceneComponent.K2_SetWorldTransform` (`self.DefaultSceneRoot`) (`KismetMathLibrary.Conv_VectorToTransform` (`/Game/Blueprint/NPCs/TeleportationPoint.Location` (`self.As Teleportation Point`))) false false))

(fn `UserConstructionScript`
  (`parent.UserConstructionScript`))