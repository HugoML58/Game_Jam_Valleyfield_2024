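; Test NPC Blueprint that talks to the player and rewards a fetch quest.
; Box overlap registers it as the player's NPC and toggles a prompt widget.
; TryDialogue opens a dialogue box and HandleDialogue advances it, choosing default, correct-item or completed-quest lines from inventory and quest state.
; Finishing the correct-item dialogue completes the quest, granting coins and souls and removing and unequipping the wanted item.
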(event `self.Box.OnComponentBeginOverlap`
  (params (OverlappedComponent :type "PrimitiveComponent Object Reference") (OtherActor :type "Actor Object Reference") (OtherComp :type "PrimitiveComponent Object Reference") (OtherBodyIndex :type Integer) (bFromSweep :type Boolean) (SweepResult :type "HitResult Structure (by ref)"))
  ;[1 1 1] Met une zone d'intéraction quand le joueur est près du NPC ou non
  (bind _asbp_player_1 (cast `/Game/Blueprint/Player/BP_Player1` OtherActor))
  (bind _output_get (set `self.Player` _asbp_player_1))
  (set `/Game/Blueprint/Player/BP_Player1.NPC` self _output_get)
  (set `self.IsClose` true)
  (`SceneComponent.SetVisibility` (`self.Widget`) true false))

(event `self.Box.OnComponentEndOverlap`
  (params (OverlappedComponent :type "PrimitiveComponent Object Reference") (OtherActor :type "Actor Object Reference") (OtherComp :type "PrimitiveComponent Object Reference") (OtherBodyIndex :type Integer))
  ;[1 1 1] Met une zone d'intéraction quand le joueur est près du NPC ou non
  (bind _asbp_player_1 (cast `/Game/Blueprint/Player/BP_Player1` OtherActor))
  (bind _output_get (set `self.Player` _asbp_player_1))
  (set `/Game/Blueprint/Player/BP_Player1.NPC` null _output_get)
  (set `self.IsClose` false)
  (`SceneComponent.SetVisibility` (`self.Widget`) false false))

(fn `ChangerDialogue`
  (params (HaveCorrectObject :type Boolean))
  (if (or (== (`self.NumeroDialogue`) (`KismetArrayLibrary.Array_Length` (`self.Dialogues`))) (and (`local.HaveCorrectObject`) (== (`self.NumeroDialogue`) (`KismetArrayLibrary.Array_Length` (`self.CorrectObjectDialogues`)))) (and (`self.HasCompletedQuest`) (== (`self.NumeroDialogue`) (`KismetArrayLibrary.Array_Length` (`self.CompletedQuestDialogues`)))))
    (`Widget.RemoveFromParent` (`self.Widget_Dialogue`))
    (set `self.IsInDialogue` false)
    (set `self.NumeroDialogue` 0)
    (set `PlayerController.bShowMouseCursor` false (`GameplayStatics.GetPlayerController` 0))
    (`/Game/Blueprint/Player/BP_Player1.IsTalking` (`self.Player`) false)
    (`SceneComponent.SetVisibility` (`self.Widget`) true false)
    (if (`self.HasCompletedQuest`)
      _
      (elif (`local.HaveCorrectObject`)
        (`self.CompleteQuest`)))
    (elif (`self.HasCompletedQuest`)
      (`self.WriteDialogue` (`self.CompletedQuestDialogues`))
      (`GameplayStatics.SpawnSound2D` "/Game/Audio/SFX/blehblerbleh-86517.blehblerbleh-86517" 1.0 1.0 0.0 null)
      (elif (`local.HaveCorrectObject`)
        (`self.WriteDialogue` (`self.CorrectObjectDialogues`))
        (`GameplayStatics.SpawnSound2D` "/Game/Audio/SFX/blehblerbleh-86517.blehblerbleh-86517" 1.0 1.0 0.0 null)
        (else
          (`self.WriteDialogue` (`self.Dialogues`))
          (`GameplayStatics.SpawnSound2D` "/Game/Audio/SFX/blehblerbleh-86517.blehblerbleh-86517" 1.0 1.0 0.0 null))))))

(fn `CheckForQuestObject`
  (returns (HasItem :type Boolean))
  (bind _hasitem (`/Game/Blueprint/Objects/Inventory/Components/BPC_Inventory.CheckForItem` (`/Game/Blueprint/Player/BP_Player1.BPC_Inventory` (`self.Player`)) (`.WantedItem_2_58BB41154E315DA8A0016B90DC7B1933` (break `/Game/Blueprint/NPCs/STRUCT_Quest` (`self.Quest`)))))
  (return _hasitem))

(fn `CompleteQuest`
  (bind _player (`self.Player`))
  (bind (_wanteditem _coinrewardamount _soulrewardamount) (break `/Game/Blueprint/NPCs/STRUCT_Quest` (`self.Quest`)))
  (set `self.HasCompletedQuest` true)
  (`/Game/Blueprint/Player/BPC_Money.addMoney` (`/Game/Blueprint/Player/BP_Player1.BPC_Money` _player) _coinrewardamount)
  (`/Game/Blueprint/Player/BP_Player1.AddSoul` _player _soulrewardamount)
  (`/Game/Blueprint/Objects/Inventory/Components/BPC_Inventory.removeItem` (`/Game/Blueprint/Player/BP_Player1.BPC_Inventory` _player) _wanteditem)
  (`/Game/Blueprint/Player/BP_Player1.Unequip Item` _player _wanteditem))

(fn `HandleDialogue`
  (if (and (`self.IsClose`) (`self.IsInDialogue`))
    (set `self.NumeroDialogue` (+ (`self.NumeroDialogue`) 1))
    (bind _hasitem (`self.CheckForQuestObject`))
    (`self.ChangerDialogue` _hasitem)))

(fn `TryDialogue`
  (if (and (`self.IsClose`) (== false (`self.IsInDialogue`)))
    (`GameplayStatics.SpawnSound2D` "/Game/Audio/SFX/blehblerbleh-86517.blehblerbleh-86517" 1.0 1.0 0.0 null)
    ;[1 1 1] What appears after the player interacts with the npc while close
    (bind _returnvalue (`|CreateWidget` "/Game/UI/WB_DialogueBox.WB_DialogueBox_C"))
    (bind _output_get (set `self.Widget_Dialogue` _returnvalue))
    (`UserWidget.AddToViewport` _output_get 0)
    (set `self.IsInDialogue` true)
    (`/Game/Blueprint/Player/BP_Player1.IsTalking` (`self.Player`) false)
    (set `PlayerController.bShowMouseCursor` true (`GameplayStatics.GetPlayerController` 0))
    (`/Game/UI/WB_DialogueBox.ChangerNom` (`self.Widget_Dialogue`) (`KismetTextLibrary.Conv_NameToText` (`self.NomNPC`)))
    (bind _hasitem (`self.CheckForQuestObject`))
    (`self.ChangerDialogue` _hasitem)
    (`SceneComponent.SetVisibility` (`self.Widget`) false false)))

(fn `UserConstructionScript`)

(fn `WriteDialogue`
  (params (Dialogue :type "Array of /Game/Blueprint/NPCs/STRUCT_Dialogue Structure"))
  (`/Game/UI/WB_DialogueBox.Changer_Dialogue` (`self.Widget_Dialogue`) (`.Dialogue_6_D298BB7742406A492CBC48B897F076EC` (break `/Game/Blueprint/NPCs/STRUCT_Dialogue` (`|GetArrayItem` Dialogue (`self.NumeroDialogue`))))))