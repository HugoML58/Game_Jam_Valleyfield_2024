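; Test quest-giver NPC that talks to the player and rewards coins and souls when they carry the wanted item.
; A box overlap enables the interact input, which opens a dialogue widget, and the continue input advances its lines.
; An inventory check and completion flag select default, correct-item or completed dialogue, with the reward granted when the correct-item conversation closes.
; Tick prints debug state on screen.
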(event `self.ReceiveBeginPlay`)

(event `self.ReceiveTick`
  (params (DeltaSeconds :type "Float (single-precision)"))
  (`KismetSystemLibrary.PrintString` (`KismetStringLibrary.Conv_BoolToString` (`self.IsClose`)) true true (struct :`G` 0.66 :`B` 1.0 :`A` 1.0) 0.0)
  (`KismetSystemLibrary.PrintString` (`KismetStringLibrary.Conv_BoolToString` (`self.IsPressed`)) true true (struct :`G` 0.66 :`B` 1.0 :`A` 1.0) 0.0)
  (`KismetSystemLibrary.PrintString` (`KismetStringLibrary.Conv_IntToString` (`self.NumeroDialogue`)) true true (struct :`G` 0.66 :`B` 1.0 :`A` 1.0) 0.0))

(event `self.Box.OnComponentBeginOverlap`
  (params (OverlappedComponent :type "PrimitiveComponent Object Reference") (OtherActor :type "Actor Object Reference") (OtherComp :type "PrimitiveComponent Object Reference") (OtherBodyIndex :type Integer) (bFromSweep :type Boolean) (SweepResult :type "HitResult Structure (by ref)"))
  ;[1 1 1] Met une zone d'intéraction quand le joueur est près du NPC ou non
  (bind _asbp_player (cast `/Game/Blueprint/Player/BP_Player` OtherActor))
  (set `self.Player` _asbp_player)
  (set `self.IsClose` true))

(event `self.Box.OnComponentEndOverlap`
  (params (OverlappedComponent :type "PrimitiveComponent Object Reference") (OtherActor :type "Actor Object Reference") (OtherComp :type "PrimitiveComponent Object Reference") (OtherBodyIndex :type Integer))
  ;[1 1 1] Met une zone d'intéraction quand le joueur est près du NPC ou non
  (bind _asbp_player (cast `/Game/Blueprint/Player/BP_Player` OtherActor))
  (set `self.Player` _asbp_player)
  (set `self.IsClose` false))

(event `EnhancedInput|/Game/TopDown/Input/Actions/IA_ContinuerDialogue`
  (params (ActionValue :type Boolean) (ElapsedSeconds :type "Float (double-precision)") (TriggeredSeconds :type "Float (double-precision)") (InputAction :type "InputAction Object Reference" :default "/Game/TopDown/Input/Actions/IA_ContinuerDialogue.IA_ContinuerDialogue"))
  (:`Started`
    (if (and (`self.IsClose`) (`self.IsInDialogue`))
      (set `self.NumeroDialogue` (+ (`self.NumeroDialogue`) 1))
      (bind _hasitem (`self.CheckForQuestObject`))
      (`self.ChangerDialogue` _hasitem))))

(event `EnhancedInput|/Game/TopDown/Input/Actions/IA_Interact`
  (params (ActionValue :type Boolean) (ElapsedSeconds :type "Float (double-precision)") (TriggeredSeconds :type "Float (double-precision)") (InputAction :type "InputAction Object Reference" :default "/Game/TopDown/Input/Actions/IA_Interact.IA_Interact"))
  (:`Started`
    (set `self.IsPressed` true)
    (if (and (`self.IsClose`) (== false (`self.IsInDialogue`)))
      ;[1 1 1] What appears after the player interacts with the npc while close
      (bind _returnvalue (`|CreateWidget` "/Game/UI/WB_DialogueBox.WB_DialogueBox_C"))
      (bind _output_get (set `self.Widget_Dialogue` _returnvalue))
      (`UserWidget.AddToViewport` _output_get 0)
      (set `self.IsInDialogue` true)
      (set `PlayerController.bShowMouseCursor` true (`GameplayStatics.GetPlayerController` 0))
      (bind _hasitem (`self.CheckForQuestObject`))
      (`self.ChangerDialogue` _hasitem)))
  (:`Completed`
    (set `self.IsPressed` false)))

(fn `ChangerDialogue`
  (params (HaveCorrectObject :type Boolean))
  (if (or (== (`self.NumeroDialogue`) (`KismetArrayLibrary.Array_Length` (`self.Dialogues`))) (and (`local.HaveCorrectObject`) (== (`self.NumeroDialogue`) (`KismetArrayLibrary.Array_Length` (`self.CorrectObjectDialogues`)))) (and (`self.HasCompletedQuest`) (== (`self.NumeroDialogue`) (`KismetArrayLibrary.Array_Length` (`self.CompletedQuestDialogues`)))))
    (`Widget.RemoveFromParent` (`self.Widget_Dialogue`))
    (set `self.IsInDialogue` false)
    (set `self.NumeroDialogue` 0)
    (set `PlayerController.bShowMouseCursor` false (`GameplayStatics.GetPlayerController` 0))
    (if (`self.HasCompletedQuest`)
      _
      (elif (`local.HaveCorrectObject`)
        (`self.CompleteQuest`)))
    (elif (`self.HasCompletedQuest`)
      (`self.WriteDialogue` (`self.CompletedQuestDialogues`))
      (elif (`local.HaveCorrectObject`)
        (`self.WriteDialogue` (`self.CorrectObjectDialogues`))
        (else
          (`self.WriteDialogue` (`self.Dialogues`)))))))

(fn `CheckForQuestObject`
  (returns (HasItem :type Boolean))
  (bind _hasite (`/Game/Blueprint/Objects/Inventory/Components/BPC_Inventory.CheckForItem` (`/Game/Blueprint/Player/BP_Player.BPC_Inventory` (`self.Player`)) (`.WantedItem_2_58BB41154E315DA8A0016B90DC7B1933` (break `/Game/STRUCT_Quest` (`self.Quest`)))))
  (return _hasite))

(fn `CompleteQuest`
  (bind _player (`self.Player`))
  (bind (_wanteditem _coinrewardamount _soulrewardamount) (break `/Game/STRUCT_Quest` (`self.Quest`)))
  (set `self.HasCompletedQuest` true)
  (`/Game/Blueprint/Player/BPC_Money.addMoney` (`/Game/Blueprint/Player/BP_Player.BPC_Money` _player) _coinrewardamount)
  (`/Game/Blueprint/Player/BP_Player.AddSoul` _player _soulrewardamount))

(fn `UserConstructionScript`)

(fn `WriteDialogue`
  (params (Dialogue :type "Array of /Game/STRUCT_Dialogue Structure"))
  (`/Game/UI/WB_DialogueBox.Changer_Dialogue` (`self.Widget_Dialogue`) (`.Dialogue_6_D298BB7742406A492CBC48B897F076EC` (break `/Game/STRUCT_Dialogue` (`|GetArrayItem` Dialogue (`self.NumeroDialogue`))))))