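; BPC_Inventory is an inventory component that holds an array of items, with debug prints as its only feedback.
; AddItem appends without a capacity check, and ShowInventory prints each entry.
; CountItems adds the array length to ItemsCount without resetting it first, then returns false and prints a full message once the total exceeds two, otherwise true.
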(fn `addItem`
  (params (item :type String))
  (`KismetArrayLibrary.Array_Add` (`self.Inventory`) item)
  (`KismetSystemLibrary.PrintString` "Hello"))

(fn `CountItems`
  (returns (IsntFull :type Boolean))
  (for _ (`self.Inventory`)
    (set `self.ItemsCount` (+ 1 (`self.ItemsCount`))))
  (if (> (`self.ItemsCount`) 2)
    (`KismetSystemLibrary.PrintString` "Inventory Full!")
    (return false)
    (else
      (return true))))

(fn `showInventory`
  (for _array_element (`self.Inventory`)
    (`KismetSystemLibrary.PrintString` _array_element)))